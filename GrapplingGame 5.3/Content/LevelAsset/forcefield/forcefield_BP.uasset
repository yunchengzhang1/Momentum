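; A forcefield actor that notifies overlapping actors implementing Forcefield_Interface by sending them a react message.
; On BeginPlay it creates a dynamic material on the Forcefield component and sets an unnamed vector parameter.
; A player-tag branch calling TestBreakthrough, which compares the overlapped actor's speed to a breakthrough threshold, is disconnected and never runs.
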(event EventBeginPlay
  (bind _returnvalue (Rendering|Material|CreateDynamicMaterialInstance (Variables|Default|Getforcefield) 0 "/Game/Materials/Forcefield_0.Forcefield_0" "None" :!class /Script/Engine.PrimitiveComponent))
  (bind _output_get (Variables|Default|SetDynamic%20Material _returnvalue))
  (Rendering|Material|SetVectorParameterValue _output_get "None" "(R=0.000000,G=0.000000,B=0.000000,A=1.000000)" :!class /Script/Engine.MaterialInstanceDynamic))

(event Collision|EventActorBeginOverlap
  (params (OtherActor :type Actor%20Object%20Reference))
  (if (Utilities|DoesObjectImplementInterface OtherActor "/Game/Interfaces/forcefield_Interface.forcefield_Interface_C")
    (bind _output_get (Variables|Default|Setoverlapped_Actor OtherActor))
    (Class|ForcefieldInterface|ReacttoForcefield(Message) _output_get)))

(event EventTick
  (params (DeltaSeconds :type Float%20%28single-precision%29)))

(fn ConstructionScript)

(fn TestBreakthrough
  (bind _overlapped_actor (Variables|Default|Getoverlapped_Actor))
  (bind _returnvalue (Transformation|GetVelocity _overlapped_actor))
  (bind _returnvalue_2 (Math|Vector|VectorLength _returnvalue))
  (Development|PrintString (Utilities|String|ToString(Float) _returnvalue_2))
  (return (> _returnvalue_2 4e+04)))