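; BP_Walker is a randomly sized enemy that drops meat when hit and becomes food on death or microwaving.
; Damage types supply health loss, armor shred, knock-up, stun and wound tallies; armor is a post-hit invulnerability window that shrinks until broken.
; Looping timers drive temperature, with burning or freezing draining health and moisture.
; On becoming food, it bubble-sorts wound tallies and passes temperature, moisture and spices through an interface.
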(event EventBeginPlay
  (CallFunction|RandomizeSize)
  (Utilities|Time|SetTimerbyFunctionName 0 "Heat or Cool?" 0.3 true)
  (Utilities|Time|SetTimerbyFunctionName 0 "ExtremeTemp?" 0.5 true))

(event EventSetMoisturebyValue
  (params (Moisture :type Float%20%28double-precision%29))
  (Variables|TempandMoist|SetMoisture (Math|Float|Clamp(Float) (+ Moisture (Variables|TempandMoist|GetMoisture)) 0.0 1e+02)))

(event Collision|EventActorEndOverlap
  (params (OtherActor :type Actor%20Object%20Reference))
  (if (Utilities|DoesObjectImplementInterface OtherActor "/Game/Environment/Temperature/AdjustTemperature.AdjustTemperature_C")
    (Class|AdjustTemperature|SetHeat(Message) OtherActor false)))

(event EventCoolforDuration
  (params (Time :type Float%20%28double-precision%29))
  (Utilities|Time|SetTimerbyFunctionName 0 "CoolDown" 0.5 true)
  (Utilities|FlowControl|Delay Time)
  (Utilities|Time|SetTimerbyFunctionName 0 "CoolDown" 0.0)
  (Variables|TempandMoist|SetCool? false))

(event EventHeatforDuration
  (params (time :type Float%20%28double-precision%29))
  (Utilities|Time|SetTimerbyFunctionName 0 "HeatUp" 0.5 true)
  (Utilities|FlowControl|Delay time)
  (Utilities|Time|SetTimerbyFunctionName 0 "HeatUp" 0.0)
  (Variables|TempandMoist|SetHeat? false))

(event EventTick
  (params (DeltaSeconds :type Float%20%28single-precision%29))
  (if (<= (Variables|BasicInfo|GetHealth) 0.0)
    (CallFunction|Death)))

(event Game|Damage|EventAnyDamage
  (params (Damage :type Float%20%28single-precision%29) (DamageType :type Damage%20Type%20Object%20Reference) (InstigatedBy :type Controller%20Object%20Reference) (DamageCauser :type Actor%20Object%20Reference))
  (Variables|DamageSystem|SetDamage%20Causer DamageCauser)
  ;[1 1 1] when armor is too low (broken)
  (if (not (Variables|DamageSystem|GetArmorBroken))
    ;[1 1 1] avoid repeated damage
    (if (Variables|DamageSystem|GetCanBeDamaged)
      (Variables|DamageSystem|SetCanBeDamaged false)
      (Utilities|Time|SetTimerbyFunctionName 0 "InvulnerabilityEnds" (Variables|DamageSystem|GetArmoredTime))
      (bind _output_get (Variables|DamageSystem|SetCurrTakenDamageType DamageType))
      (bind (_damage_out _posturedamage _armorshred _knockup _stunduration _meatchance _soundplays _woundname) (Class|DamageTypeBPI|ProcessDamage(Message) _output_get Damage))
      (TakingDamage|LoseArmor _armorshred)
      (TakingDamage|LoseHealth _damage_out)
      (TakingDamage|DropMeat _meatchance)
      (TakingDamage|KnockUp _knockup)
      (CallFunction|InjuryFX _soundplays)
      (CallFunction|SetStun _stunduration)
      (Cooking|AddWoundType _woundname)
      (Class|AfterLandingAttack|MovementSlow(Message) (Variables|DamageSystem|GetDamage%20Causer) :!label _label)
      (Class|AfterLandingAttack|ReceiveEnemyInfo(Message) (Variables|DamageSystem|GetDamage%20Causer) (Utilities|Struct|MakeEnemyInfo "Walker" (/ (Variables|BasicInfo|GetHealth) (Variables|BasicInfo|GetMaxHealth)) false (/ (Variables|DamageSystem|GetArmoredTime) (Variables|BasicInfo|GetMax_ArmoredTime))))
      (Development|PrintString _woundname true true "(R=0.000000,G=0.660000,B=1.000000,A=1.000000)" 8.0))
    (else
      (bind _output_get_2 (Variables|DamageSystem|SetCurrTakenDamageType DamageType))
      (bind (_damage_out_2 _posturedamage_2 _armorshred_2 _knockup_2 _stunduration_2 _meatchance_2 _soundplays_2 _woundname_2) (Class|DamageTypeBPI|ProcessDamage(Message) _output_get_2 Damage))
      (TakingDamage|LoseHealth _damage_out_2)
      (TakingDamage|DropMeat _meatchance_2)
      (CallFunction|InjuryFX _soundplays_2)
      (CallFunction|SetStun _stunduration_2)
      (Cooking|AddWoundType _woundname_2)
      (goto _label))))

(event EventLongGrunt
  (bind _size (Variables|BasicInfo|GetSize))
  (bind _returnvalue (/ 1.0 _size))
  (Audio|PlaySoundatLocation "/Game/Enemies/walker/Audio/long_grunt.long_grunt" (Transformation|GetActorLocation) "0, 0, 0" _returnvalue _returnvalue 0.0 0 0 0 0))

(event EventGrunt
  (bind _size (Variables|BasicInfo|GetSize))
  (bind _returnvalue (/ 1.0 _size))
  (Audio|PlaySoundatLocation "/Game/Enemies/walker/Audio/grunt1.grunt1" (Transformation|GetActorLocation) "0, 0, 0" _returnvalue _returnvalue 0.0 0 0 0 0))

(event EventSetCool
  (params (CoolDown? :type Boolean))
  (Utilities|Time|SetTimerbyFunctionName 0 "CoolDown" 0.5 CoolDown?)
  ;[1 1 1] if true, do nothing
  ; if false, heat == false
  (Utilities|FlowControl|Delay 0.7)
  (if (not CoolDown?)
    (Variables|TempandMoist|SetCool? false)))

(event EventSetHeat
  (params (HeatUp? :type Boolean))
  (Utilities|Time|SetTimerbyFunctionName 0 "HeatUp" 0.5 HeatUp?)
  ;[1 1 1] if true, do nothing
  ; if false, heat == false
  (Utilities|FlowControl|Delay 0.7)
  (if (not HeatUp?)
    (Variables|TempandMoist|SetHeat? false)))

(event EventActivateMicrowave
  (Microwave|MicrowaveCooking)
  (bind _returnvalue (Game|SpawnActorfromClass "/Game/Consumable/Food/Food_Prototype.Food_Prototype_C" (Math|Transform|MakeTransform (Transformation|GetActorLocation) "0, 0, 0" (Math|Conversions|ToVector(Float) (Variables|BasicInfo|GetSize))) "AlwaysSpawn" self 0))
  (Microwave|OutputtoFood _returnvalue)
  (Actor|DestroyActor))

(event Collision|EventActorBeginOverlap
  (params (OtherActor :type Actor%20Object%20Reference))
  (TempAndMoist|TemperatureAura? OtherActor))

(fn ConstructionScript)

(fn InvulnerabilityEnds
  (Variables|DamageSystem|SetCanBeDamaged true))

(fn LoseArmor
  (params (ShredIn :type Float%20%28double-precision%29))
  (Variables|DamageSystem|SetArmoredTime (/ (Variables|DamageSystem|GetArmoredTime) ShredIn))
  (if (not (>= (Variables|DamageSystem|GetArmoredTime) 1e-05))
    (Variables|DamageSystem|SetArmorBroken true)
    (Audio|PlaySound2D "/Game/DamageType/DamageAudio/bonebreak.bonebreak" 1.0 1.0 0.0 0 0)
    (Development|PrintString "ArmorBreak!" true true "(R=1.000000,G=0.534225,B=0.000000,A=1.000000)")))

(fn KnockUp
  (params (KnockUp%20Strength :type Float%20%28double-precision%29))
  (bind _charactermovement (Variables|Character|GetCharacterMovement))
  (if (> KnockUp%20Strength 0.0)
    (Variables|/Script/Engine.MovementComponent|SetVelocity _charactermovement "0, 0, 0")
    (Physics|AddImpulse _charactermovement (Math|Vector|MakeVector 0.0 0.0 KnockUp%20Strength) false)))

(fn DropMeat
  (params (MeatChance :type Integer))
  (if (>= MeatChance (Math|Random|RandomIntegerinRange 1 100))
    (Game|SpawnActorfromClass "/Game/Consumable/Food/Food_Prototype.Food_Prototype_C" (Math|Transform|MakeTransform (Transformation|GetWorldLocation (Variables|Default|Getwalker_eyeball)) "0, 0, 0" (Math|Conversions|ToVector(Float) (Variables|BasicInfo|GetSize))) "AlwaysSpawn" self 0)))

(fn LoseHealth
  (params (DamageIn :type Float%20%28double-precision%29))
  (Variables|BasicInfo|SetHealth (- (Variables|BasicInfo|GetHealth) DamageIn)))

(fn AddSpiceType
  (params (spice%20type :type String))
  (bind _spiceregister_value (Variables|CookingParams|GetSpiceRegister_Value))
  (bind _spiceregister_name (Variables|CookingParams|GetSpiceRegister_Name))
  (bind _returnvalue (Utilities|Array|FindItem _spiceregister_name spice%20type))
  (if (Utilities|Array|IsValidIndex _spiceregister_name _returnvalue)
    (Utilities|Array|SetArrayElem _spiceregister_value _returnvalue (+ (Utilities|Array|Get(acopy) _spiceregister_value _returnvalue) 1))
    (else
      (Development|PrintString "Cooking - AddSpiceType - Index Error!" true true "(R=1.000000,G=0.000000,B=0.036710,A=1.000000)" 6.0))))

(fn Death
  (Audio|PlaySound2D "/Game/Enemies/walker/Audio/bubble_death_short.bubble_death_short" 1.0 1.0 0.0 0 self)
  (Microwave|MicrowaveCooking)
  (bind _returnvalue (Game|SpawnActorfromClass "/Game/Consumable/Food/Food_Prototype.Food_Prototype_C" (Math|Transform|MakeTransform (Transformation|GetActorLocation) "0, 0, 0" (Math|Conversions|ToVector(Float) (Variables|BasicInfo|GetSize))) "AlwaysSpawn" self 0))
  (Microwave|OutputtoFood _returnvalue)
  (Class|AfterLandingAttack|ReceiveEnemyInfo(Message) (Game|GetPlayerCharacter 0) (Utilities|Struct|MakeEnemyInfo "" 0.0 false 0.0))
  (Actor|DestroyActor))

(fn InjuryFX
  (params (DamageSound :type Sound%20Wave%20Object%20Reference))
  (if (Variables|DamageSystem|GetCanPlayInjuryFX)
    (Variables|DamageSystem|SetCanPlayInjuryFX false)
    (Utilities|Time|SetTimerbyFunctionName 0 "EnableInjuryFX" (Variables|DamageSystem|GetInjuryFXCooldown))
    (Audio|PlaySoundatLocation DamageSound (Transformation|GetSocketLocation (Variables|Character|GetMesh) "None") "0, 0, 0" 1.0 1.0 0.0 0 0 0 0)))

(fn EnableInjuryFX
  (Variables|DamageSystem|SetCanPlayInjuryFX true))

(fn SetStun
  (params (StunDuration :type Float%20%28double-precision%29))
  (if (not (Variables|AIStatus|GetisStunned))
    (if (> StunDuration 0.0)
      (Variables|AIStatus|SetisStunned true)
      (Utilities|Time|SetTimerbyFunctionName 0 "DisableStun" StunDuration)
      (return))))

(fn DisableStun
  (Variables|AIStatus|SetisStunned false))

(fn BubbleSort
  (params (value :type Array%20of%20Integers) (name :type Array%20of%20Strings))
  (Variables|CookingParams|Setbubble_N (Utilities|Array|Length value))
  (while (> (Variables|CookingParams|Getbubble_N) 1)
    (Variables|CookingParams|Setbubble_newN 0)
    (for _index (range 1 (- (Variables|CookingParams|Getbubble_N) 1))
      (if (< (Utilities|Array|Get(acopy) value (- _index 1)) (Utilities|Array|Get(acopy) value _index))
        (Utilities|Array|Swap value (- _index 1) _index)
        (Utilities|Array|Swap name (- _index 1) _index)
        (Variables|CookingParams|Setbubble_newN _index)))
    (Variables|CookingParams|Setbubble_N (Variables|CookingParams|Getbubble_newN))))

(fn OutputtoFood
  (params (FoodDrop :type Actor%20Object%20Reference%20%28by%20ref%29))
  (if (Utilities|DoesObjectImplementInterface FoodDrop "/Game/Consumable/Food/FoodInput.FoodInput_C")
    (for (_array_element _array_index) (Variables|CookingParams|GetSpiceRegister_Value)
      ;[1 1 1] if flavor/spice > 0, add into the output array
      (if (> _array_element 0)
        (Utilities|Array|Add (Variables|CookingParams|GetSpiceOutput) _array_index)))
    (Class|FoodInput|LetEmCook(Message) FoodDrop (Variables|TempandMoist|GetTemperature) (Variables|TempandMoist|GetMoisture) (Variables|CookingParams|GetSpiceOutput))))

(fn MicrowaveCooking
  (params (Other%20Actor :type Actor%20Object%20Reference))
  (utility|BubbleSort (Variables|CookingParams|GetWoundRegister_Value) (Variables|CookingParams|GetWoundRegister_Name))
  (utility|BubbleSort (Variables|CookingParams|GetWoundRegister_Value) (Variables|CookingParams|GetSpiceRegister_Name))
  (if (Utilities|Array|ContainsItem (Variables|CookingParams|GetSpiceRegister_Value) 1)
    _))

(fn AddWoundType
  (params (wound%20type :type String))
  (bind _woundregister_name (Variables|CookingParams|GetWoundRegister_Name))
  (bind _woundregister_value (Variables|CookingParams|GetWoundRegister_Value))
  (bind _returnvalue (Utilities|Array|FindItem _woundregister_name wound%20type))
  (if (Utilities|Array|IsValidIndex _woundregister_name _returnvalue)
    (Utilities|Array|SetArrayElem _woundregister_value _returnvalue (+ (Utilities|Array|Get(acopy) _woundregister_value _returnvalue) 1))
    (else
      (Development|PrintString "Add Wound Type - Index Error!" true true "(R=1.000000,G=0.000000,B=0.036710,A=1.000000)" 6.0)
      (Development|PrintString wound%20type true true "(R=1.000000,G=0.000000,B=0.036710,A=1.000000)" 6.0))))

(fn HeatUp
  (Variables|TempandMoist|SetHeat? true)
  (Development|PrintString "HEAT UP" true true "(R=1.000000,G=0.582378,B=0.000000,A=1.000000)" 1.0))

(fn CoolDown
  (Variables|TempandMoist|SetCool? true))

(fn HeatorCool?
  (bind _temp_adjust_rate (Variables|TempandMoist|GetTemp%20Adjust%20Rate))
  ;[1 1 1] XOR 1: 01 or 10, find if chill or heat
  ; XOR 0: 00 or 11, recover temp
  (if (Class|KismetMathLibrary|XORBoolean (Variables|TempandMoist|GetCool?) (Variables|TempandMoist|GetHeat?))
    ;[1 1 1] if chill ==1, 10
    ; if chill ==0, 01
    (if (Variables|TempandMoist|GetCool?)
      ;[1 1 1] cool down:  temp-= (cooldown rate)
      (bind _output_get (Variables|TempandMoist|SetTemperature (Math|Float|Clamp(Float) (- (Variables|TempandMoist|GetTemperature) (Variables|TempandMoist|GetCoolDown%20Scale)) 0.0 1e+02)))
      (else
        ;[1 1 1] heating up: temp+= (heatup rate)
        (bind _output_get_2 (Variables|TempandMoist|SetTemperature (Math|Float|Clamp(Float) (+ (Variables|TempandMoist|GetTemperature) (Variables|TempandMoist|GetHeatUp%20Scale)) 0.0 1e+02)))))
    ;[1 1 1] update when status status is being applied
    (Class|AfterLandingAttack|ReceiveEnemyInfo(Message) (Variables|DamageSystem|GetDamage%20Causer) (Utilities|Struct|MakeEnemyInfo "Walker" (/ (Variables|BasicInfo|GetHealth) (Variables|BasicInfo|GetMaxHealth)) false (/ (Variables|DamageSystem|GetArmoredTime) (Variables|BasicInfo|GetMax_ArmoredTime))))
    (elif (not (== (Variables|TempandMoist|GetTemp%20Default) (Variables|TempandMoist|GetTemperature)))
      ;[1 1 1] increase/reduce (curr temp) towards the (default temperature) by (temperature adjust rate)
      (bind _output_get_3 (Variables|TempandMoist|SetTemperature (+ (Variables|TempandMoist|GetTemperature) (Math|Float|Clamp(Float) (- (Variables|TempandMoist|GetTemp%20Default) (Variables|TempandMoist|GetTemperature)) (* _temp_adjust_rate -1.0) _temp_adjust_rate))))
      ;[1 1 1] print temperature status
      (Development|PrintString (Utilities|String|ToString(Float) _output_get_3) true true "(R=0.000000,G=1.000000,B=0.001688,A=1.000000)" 0.3))))

(fn ExtremeTemp?
  ;[1 1 1] if temperature ==
  ; 100, apply burn effect
  ; 0, apply freeze effect
  ; else, do nothing
  ;[1 1 1] react to temperature based on condition
  ;;[1 1 1] if unit curr temperature >= burn bound
  (if (>= (Variables|TempandMoist|GetTemperature) (Variables|TempandMoist|GetBurn%20Bound))
    ;;[1 1 1] apply burn damage, freeze effect,  reduce moisture on tick
    (TakingDamage|LoseHealth 1.0)
    (Variables|TempandMoist|SetMoisture (- (Variables|TempandMoist|GetMoisture) 2.0))
    ;[1 1 1] then set niagara to CatchFlame
    (Class|NiagaraComponent|SetAsset (Variables|Default|GetTemperature%20Niagara%20Emitter) "/Game/Niagara/CatchFlame/Walker_CatchFlame.Walker_CatchFlame" true)
    (Variables|TempandMoist|SetHeat%20Scale 2)
    (else
      ;;[1 1 1] if unit curr temperature <= freeze bound
      (if (<= (Variables|TempandMoist|GetTemperature) (Variables|TempandMoist|GetFreeze%20Bound))
        ;;[1 1 1] apply freeze damage, freeze effect, and reduct moisture
        (TakingDamage|LoseHealth 1.0)
        (Variables|TempandMoist|SetMoisture (- (Variables|TempandMoist|GetMoisture) 2.0))
        ;[1 1 1] then set niagara to CatchFrost
        (Class|NiagaraComponent|SetAsset (Variables|Default|GetTemperature%20Niagara%20Emitter) "/Game/Niagara/CatchFrost/Walker_CatchFrost.Walker_CatchFrost" true)
        (Variables|TempandMoist|SetHeat%20Scale 1)
        (else
          ;[1 1 1] then set niagara to DEFAULT
          (Class|NiagaraComponent|SetAsset (Variables|Default|GetTemperature%20Niagara%20Emitter) 0 true)
          (Variables|TempandMoist|SetHeat%20Scale 0))))))

(fn RandomizeSize
  (bind _output_get (Variables|BasicInfo|SetSize (Math|Random|RandomFloatinRange 0.5 1.5)))
  (Transformation|SetActorScale3D (Math|Conversions|ToVector(Float) _output_get))
  (bind _output_get_2 (Variables|BasicInfo|SetMaxHealth (* _output_get (Variables|BasicInfo|GetMaxHealth))))
  (Variables|BasicInfo|SetHealth _output_get_2))

(fn BecomeHeatSource?
  ;[1 1 1] if temperature is higher than Burn Bound: target is burning
  (if (>= (Variables|TempandMoist|GetTemperature) (Variables|TempandMoist|GetBurn%20Bound))
    (Class|NiagaraComponent|SetAsset (Variables|Default|GetTemperature%20Niagara%20Emitter) "/Game/Niagara/CatchFlame/Walker_CatchFlame.Walker_CatchFlame" true)))

(fn BecomeCoolSource?
  ;[1 1 1] if temperature is lower than Freeze Bound: target is freezing
  (if (<= (Variables|TempandMoist|GetTemperature) (Variables|TempandMoist|GetFreeze%20Bound))
    (Class|NiagaraComponent|SetAsset (Variables|Default|GetTemperature%20Niagara%20Emitter) "/Game/Niagara/CatchFrost/Walker_CatchFrost.Walker_CatchFrost" true)))

(fn TemperatureAura?
  (params (Other%20Actor :type Actor%20Object%20Reference))
  (if (Utilities|DoesObjectImplementInterface 0 "/Game/Environment/Temperature/AdjustTemperature.AdjustTemperature_C")
    (switch int 0
      (:1
        (Class|AdjustTemperature|SetHeat(Message) Other%20Actor true))
      (:2
        (Class|AdjustTemperature|SetCool(Message) Other%20Actor true)))
    (return)))

(fn ShouldMicrowave?
  (return (<= (/ (Variables|BasicInfo|GetHealth) (Variables|BasicInfo|GetMaxHealth)) 0.99)))