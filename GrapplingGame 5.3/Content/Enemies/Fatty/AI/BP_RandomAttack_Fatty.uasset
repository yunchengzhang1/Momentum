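; Behavior tree task that picks a random attack type for the Fatty enemy when its chase target is in range.
; It measures the distance from the controlled BP_Fatty to the ChaseTarget blackboard actor.
; Within the hardcoded range it sets AttackType on the pawn to one of three random values and succeeds.
; Out of range it prints the distance and fails, and it also fails if the pawn cast fails.
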(event EventReceiveExecuteAI
  (params (OwnerController :type AI%20Controller%20Object%20Reference) (ControlledPawn :type Pawn%20Object%20Reference))
  (bind _asbp_fatty (Utilities|Casting|CastToBP_Fatty ControlledPawn)
    (:then
      (if (<= (Math|Vector|VectorLength (- (Transformation|GetActorLocation (AI|BehaviorTree|GetBlackboardValueasActor (Variables|Default|GetChaseTarget))) (Transformation|GetActorLocation _asbp_fatty))) 1e+03)
        (Variables|/Game/Enemies/Fatty/BP_Fatty.BP_Fatty_C|SetAttackType? _asbp_fatty (Math|Random|RandomIntegerinRange 0 2))
        (AI|BehaviorTree|FinishExecute true)
        (else
          (Development|PrintString (Utilities|String|ToString(Float) (Math|Vector|VectorLength (- (Transformation|GetActorLocation (AI|BehaviorTree|GetBlackboardValueasActor (Variables|Default|GetChaseTarget))) (Transformation|GetActorLocation _asbp_fatty)))))
          (AI|BehaviorTree|FinishExecute false :!label _label))))
    (:CastFailed
      (goto _label))))