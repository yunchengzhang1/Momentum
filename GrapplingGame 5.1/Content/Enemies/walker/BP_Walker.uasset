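; Walker enemy character that takes damage, drops sushi pickups and destroys itself when Tick finds its health depleted.
; AnyDamage asks the DamageType, via ProcessDamageMessage, for damage, armor shred, drop chance, knock-up and sound, then messages the causer to slow movement.
; Armor is a post-hit invulnerability window that each shred divides until it breaks, after which hits always land without knock-up.
; Injury sounds have their own cooldown.
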(event EventBeginPlay)

(event Collision|EventActorBeginOverlap
  (params (OtherActor :type Actor%20Object%20Reference)))

(event EventTick
  (params (DeltaSeconds :type Float%20%28single-precision%29))
  (if (<= (Variables|Default|GetHealth) 0.0)
    (CallFunction|Death)))

(event Game|Damage|EventAnyDamage
  (params (Damage :type Float%20%28single-precision%29) (DamageType :type Damage%20Type%20Object%20Reference) (InstigatedBy :type Controller%20Object%20Reference) (DamageCauser :type Actor%20Object%20Reference))
  ;[1 1 1] when armor is too low (broken)
  (if (not (Variables|Default|GetArmorBroken))
    ;[1 1 1] avoid repeated damage
    (if (Variables|Default|GetCanBeDamaged)
      (Variables|Default|SetCanBeDamaged false)
      (Utilities|Time|SetTimerbyFunctionName 0 "InvulnerabilityEnds" (Variables|Default|GetArmoredTime))
      (bind _output_get (Variables|Default|SetCurrTakenDamageType DamageType))
      (bind (_damage_out _posturedamage _meatchance _armorshred _knockup _soundplays) (Class|DamageTypeBPI|ProcessDamage(Message) _output_get Damage))
      (CallFunction|LoseArmor _armorshred)
      (CallFunction|LoseHealth _damage_out)
      (CallFunction|DropMeat _meatchance)
      (CallFunction|KnockUp _knockup)
      (CallFunction|InjuryFX _soundplays)
      (Class|AfterLandingAttack|MovementSlow(Message) DamageCauser :!label _label))
    (else
      (bind _output_get_2 (Variables|Default|SetCurrTakenDamageType DamageType))
      (bind (_damage_out_2 _posturedamage_2 _meatchance_2 _armorshred_2 _knockup_2 _soundplays_2) (Class|DamageTypeBPI|ProcessDamage(Message) _output_get_2 Damage))
      (CallFunction|LoseHealth _damage_out_2)
      (CallFunction|DropMeat _meatchance_2)
      (CallFunction|InjuryFX _soundplays_2)
      (goto _label))))

(fn ConstructionScript)

(fn InvulnerabilityEnds
  (Variables|Default|SetCanBeDamaged true))

(fn DropMeat
  (params (MeatChance :type Integer))
  (if (>= MeatChance (Math|Random|RandomIntegerinRange 1 100))
    (Game|SpawnActorfromClass "/Game/Consumable/Sushi_TunaAkami.Sushi_TunaAkami_C" (Math|Conversions|ToTransform(Vector) (Transformation|GetWorldLocation (Variables|Default|Getwalker_eyeball))) "AlwaysSpawn" 0 0)))

(fn LoseHealth
  (params (DamageIn :type Float%20%28double-precision%29))
  (Variables|Default|SetHealth (- (Variables|Default|GetHealth) DamageIn)))

(fn LoseArmor
  (params (ShredIn :type Float%20%28double-precision%29))
  (Variables|Default|SetArmoredTime (/ (Variables|Default|GetArmoredTime) ShredIn))
  (if (not (>= (Variables|Default|GetArmoredTime) 1e-05))
    (Variables|Default|SetArmorBroken true)
    (Audio|PlaySound2D "/Game/DamageType/DamageAudio/bonebreak.bonebreak" 1.0 1.0 0.0 0 0)
    (Development|PrintString "ArmorBreak!" true true "(R=1.000000,G=0.534225,B=0.000000,A=1.000000)")))

(fn KnockUp
  (params (KnockUp%20Strength :type Float%20%28double-precision%29))
  (bind _charactermovement (Variables|Character|GetCharacterMovement))
  (Variables|/Script/Engine.MovementComponent|SetVelocity _charactermovement "0, 0, 0")
  (Physics|AddImpulse _charactermovement (Math|Vector|MakeVector 0.0 0.0 KnockUp%20Strength) false))

(fn Death
  (bind _self self)
  (Audio|PlaySound2D "/Game/Enemies/walker/Audio/bubble_death_short.bubble_death_short" 1.0 1.0 0.0 0 _self)
  (Game|SpawnActorfromClass "/Game/Consumable/Sushi_TunaOtoro.Sushi_TunaOtoro_C" (Math|Conversions|ToTransform(Vector) (Transformation|GetActorLocation)) "AlwaysSpawn" _self 0)
  (Actor|DestroyActor))

(fn InjuryFX
  (params (DamageSound :type Sound%20Wave%20Object%20Reference))
  (if (Variables|Default|GetCanPlayInjuryFX)
    (Variables|Default|SetCanPlayInjuryFX false)
    (Utilities|Time|SetTimerbyFunctionName 0 "EnableInjuryFX" (Variables|Default|GetInjuryFXCooldown))
    (Audio|PlaySoundatLocation DamageSound (Transformation|GetSocketLocation (Variables|Character|GetMesh) "None") "0, 0, 0" 1.0 1.0 0.0 0 0 0 0)))

(fn EnableInjuryFX
  (Variables|Default|SetCanPlayInjuryFX true))