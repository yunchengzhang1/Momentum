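; BP_RandomAttack is a Behavior Tree task that makes a BP_Walker enemy perform a randomly chosen kick or slap.
; It sets EnemySpotted, turns on either IsKicking or IsSlapping by coin flip, then clears both after a fixed delay and finishes successfully.
; If the controlled pawn is not a Walker, it prints the ChaseTarget blackboard actor's name and fails.
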(event EventReceiveExecuteAI
  (params (OwnerController :type AI%20Controller%20Object%20Reference) (ControlledPawn :type Pawn%20Object%20Reference))
  (bind _asbp_walker (Utilities|Casting|CastToBP_Walker ControlledPawn)
    (:then
      (Variables|/Game/Enemies/walker/BP_Walker.BP_Walker_C|SetenemySpotted _asbp_walker true)
      (bind _output_get (Variables|Default|SetRandomBool (Math|Random|RandomBool)))
      (Variables|/Game/Enemies/walker/BP_Walker.BP_Walker_C|SetisKicking _asbp_walker _output_get)
      (Variables|/Game/Enemies/walker/BP_Walker.BP_Walker_C|SetisSlapping _asbp_walker (not _output_get))
      (Utilities|FlowControl|Delay 2.0)
      (Variables|/Game/Enemies/walker/BP_Walker.BP_Walker_C|SetisKicking _asbp_walker false)
      (Variables|/Game/Enemies/walker/BP_Walker.BP_Walker_C|SetisSlapping _asbp_walker false)
      (AI|BehaviorTree|FinishExecute true))
    (:CastFailed
      (Development|PrintString (Utilities|GetDisplayName (AI|BehaviorTree|GetBlackboardValueasActor (Variables|Default|GetChaseTarget))))
      (AI|BehaviorTree|FinishExecute false))))