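; Enemy character Blueprint for Fatty, holding combat-state functions for damage, armor shred and break, knock-up, timed stun and ending invulnerability.
; A health-ratio check sets the fight phase with debug prints, calling Phase1Start on the Fatty AI controller for phase one.
; Injury sounds are rate-limited by a cooldown timer.
; Meat drops spawn tuna sushi by chance, while death always spawns otoro and destroys the actor.
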(fn ConstructionScript)

(fn InvulnerabilityEnds
  (Variables|Default|SetCanBeDamaged true))

(fn DropMeat
  (params (MeatChance :type Integer))
  (if (>= MeatChance (Math|Random|RandomIntegerinRange 1 100))
    (Game|SpawnActorfromClass "/Game/Consumable/Sushi_TunaAkami.Sushi_TunaAkami_C" (Math|Transform|MakeTransform (Transformation|GetWorldLocation (Variables|Character|GetMesh))) "AlwaysSpawn" self 0)))

(fn LoseHealth
  (params (DamageIn :type Float%20%28double-precision%29))
  (Variables|Default|SetCurrHealth (- (Variables|Default|GetCurrHealth) DamageIn)))

(fn LoseArmor
  (params (ShredIn :type Float%20%28double-precision%29))
  (Variables|Default|SetArmoredTime (/ (Variables|Default|GetArmoredTime) ShredIn))
  (if (not (>= (Variables|Default|GetArmoredTime) 1e-05))
    (Variables|Default|SetArmorBroken true)
    (Audio|PlaySound2D "/Game/DamageType/DamageAudio/bonebreak.bonebreak" 1.0 1.0 0.0 0 0)
    (Development|PrintString "ArmorBreak!" true true "(R=1.000000,G=0.534225,B=0.000000,A=1.000000)")))

(fn KnockUp
  (params (KnockUp%20Strength :type Float%20%28double-precision%29))
  (bind _charactermovement (Variables|Character|GetCharacterMovement))
  (Variables|/Script/Engine.MovementComponent|SetVelocity _charactermovement "0, 0, 0")
  (Physics|AddImpulse _charactermovement (Math|Vector|MakeVector 0.0 0.0 KnockUp%20Strength) false))

(fn Death
  (bind _self self)
  (Audio|PlaySound2D "/Game/Enemies/walker/Audio/bubble_death_short.bubble_death_short" 1.0 1.0 0.0 0 _self)
  (Game|SpawnActorfromClass "/Game/Consumable/Sushi_TunaOtoro.Sushi_TunaOtoro_C" (Math|Transform|MakeTransform (Transformation|GetActorLocation)) "AlwaysSpawn" _self 0)
  (Actor|DestroyActor))

(fn InjuryFX
  (params (DamageSound :type Sound%20Wave%20Object%20Reference))
  (if (Variables|Default|GetCanPlayInjuryFX)
    (Variables|Default|SetCanPlayInjuryFX false)
    (Utilities|Time|SetTimerbyFunctionName 0 "EnableInjuryFX" (Variables|Default|GetInjuryFXCooldown))
    (Audio|PlaySoundatLocation DamageSound (Transformation|GetSocketLocation (Variables|Character|GetMesh) "None") "0, 0, 0" 1.0 1.0 0.0 0 0 0 0)))

(fn EnableInjuryFX
  (Variables|Default|SetCanPlayInjuryFX true))

(fn SetStun
  (params (StunDuration :type Float%20%28double-precision%29))
  (if (not (Variables|Default|GetisStunned))
    (if (> StunDuration 0.0)
      (Variables|Default|SetisStunned true)
      (Utilities|Time|SetTimerbyFunctionName 0 "DisableStun" StunDuration)
      (return))))

(fn DisableStun
  (Variables|Default|SetisStunned false))

(fn PhaseTransition
  (bind _currhealth (Variables|Default|GetCurrHealth))
  (bind _maxhealth (Variables|Default|GetMaxHealth))
  (bind _returnvalue (/ _currhealth _maxhealth))
  (if (<= _returnvalue 0.98)
    (if (> _returnvalue 0.96)
      (Variables|Default|SetPhase? 1)
      (Development|PrintString "PHASE 1" true true "(R=0.000000,G=0.074137,B=1.000000,A=1.000000)")
      (Utilities|FlowControl|DoOnce false
        (:Completed
          (bind _asaibp_fatty (Utilities|Casting|CastToAIBP_Fatty (AI|GetAIController self)))
          (Default|Phase1Start _asaibp_fatty)))
      (else
        (Variables|Default|SetPhase? 2)
        (Development|PrintString "PHASE 2" true true "(R=1.000000,G=0.648792,B=0.000000,A=1.000000)")))
    (else
      (Development|PrintString "HIT ME MORE TO GET PHASE 1" true true "(R=1.000000,G=0.000000,B=0.006324,A=1.000000)"))))