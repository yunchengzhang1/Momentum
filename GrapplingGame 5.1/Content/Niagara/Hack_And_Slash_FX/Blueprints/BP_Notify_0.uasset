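; BP_Notify_0 is an anim notify state that spawns a selectable Niagara effect when its window begins.
; The effect spawns unattached at the mesh's EffectSocket, with a world-space position offset and a rotation combined with the socket's.
; Its scale grows with the square root of player 0's movement speed, read from that character even if another mesh plays the animation.
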(fn ReceivedNotifyBegin
  (params (MeshComp :type Skeletal%20Mesh%20Component%20Object%20Reference) (Animation :type Anim%20Sequence%20Base%20Object%20Reference) (TotalDuration :type Float%20%28single-precision%29) (EventReference :type Anim%20Notify%20Event%20Reference%20Structure%20%28by%20ref%29))
  (Niagara|SpawnSystematLocation MeshComp (Variables|Default|GetNiagara%20System%20Select) (+ (Transformation|GetSocketLocation MeshComp "EffectSocket") (Variables|Default|GetFX_Offset)) (Math|Rotator|CombineRotators (Transformation|GetSocketRotation MeshComp "EffectSocket") (Variables|Default|GetFX_Rotation)) (* "4.000000,4.000000,4.000000" (+ (Math|Float|Sqrt (* (Math|Vector|VectorLength (Variables|/Script/Engine.MovementComponent|GetVelocity (Variables|/Script/Engine.Character|GetCharacterMovement (Game|GetPlayerCharacter MeshComp)))) 0.07)) 1.0)))
  (return false))